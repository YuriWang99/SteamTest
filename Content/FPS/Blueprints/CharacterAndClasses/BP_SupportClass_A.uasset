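; BP_SupportClass_A is a Support class character Blueprint whose throwable item is a small explosive ammo box.
; ThrowItem passes that box class to ServerSpawnMedKit to spawn it.
; Equipping plays the weapon's first-person montage, shows the weapon on a short timer to avoid a one-frame misplacement, and clears PerformingAction on completion.
; Unequipping plays its montage at double speed and hides the weapon on blend out.
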(event `/Game/FPS/Blueprints/Interfaces/iPawnActions.ThrowItem`
  (`self.Server_SpawnMedKit` "/Game/FPS/Blueprints/AmmoBox/BP_SmallExplosiveAmmoBox.BP_SmallExplosiveAmmoBox_C"))

(fn `UserConstructionScript`
  (`parent.UserConstructionScript`))