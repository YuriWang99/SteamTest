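; Game state for the Capture the Flag mode that tracks both team flags and handles carriers leaving the match.
; GetObjectives gathers every BP_BaseFlag actor as the objectives and assigns each to the team 0 or team 1 flag slot by its Team value.
; On player logout, it drops any flag still marked as taken whose carrier is no longer valid, so a departed player cannot keep it.
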(event `self.GetObjectives`
  (bind _outactors (`GameplayStatics.GetAllActorsOfClass` "/Game/FPS/Blueprints/GameObjectives/CTF_Flag/BP_BaseFlag.BP_BaseFlag_C"))
  (set `self.Objectives` _outactors)
  (for _array_element _outactors
    (if (`KismetMathLibrary.Conv_IntToBool` (`/Game/FPS/Blueprints/GameObjectives/CTF_Flag/BP_BaseFlag.Team` _array_element))
      (set `self.FlagTeam_1` _array_element)
      (else
        (set `self.FlagTeam_0` _array_element)))))

(event `self.HandlePlayerLogout`
  (params (PlayerController :type "PlayerController Object Reference"))
  (for _array_element (`|MakeArray` (`self.FlagTeam_1`) (`self.FlagTeam_0`))
    (`/Game/FPS/Blueprints/GameObjectives/CTF_Flag/BP_BaseFlag.Carrier` _array_element
      (:`then`)
      (:`else`
        (if (`/Game/FPS/Blueprints/GameObjectives/CTF_Flag/BP_BaseFlag.bFlagTaken` _array_element)
          (`/Game/FPS/Blueprints/GameObjectives/CTF_Flag/BP_BaseFlag.DropFlag` _array_element))))))

(fn `UserConstructionScript`
  (`parent.UserConstructionScript`))